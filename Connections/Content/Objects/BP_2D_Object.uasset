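; BP_2D_Object is a pickup item shown as a flat plane that turns to face the player's camera.
; Each tick it sets the plane's yaw from a look-at toward the third-person character's FollowCamera, a yaw-only billboard effect.
; Sphere overlap begin and end show and hide its widget.
; PickUpItem prints a message, triggers DestroyItem to remove the actor after a short delay, and returns the Item.
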(event `Destroy Item`
  (`KismetSystemLibrary.Delay` 0.1)
  (`self.K2_DestroyActor`))

(event `self.Sphere.OnComponentBeginOverlap`
  (params (OverlappedComponent :type "PrimitiveComponent Object Reference") (OtherActor :type "Actor Object Reference") (OtherComp :type "PrimitiveComponent Object Reference") (OtherBodyIndex :type Integer) (bFromSweep :type Boolean) (SweepResult :type "HitResult Structure (by ref)"))
  (`SceneComponent.SetVisibility` (`self.Widget`) true false))

(event `self.Sphere.OnComponentEndOverlap`
  (params (OverlappedComponent :type "PrimitiveComponent Object Reference") (OtherActor :type "Actor Object Reference") (OtherComp :type "PrimitiveComponent Object Reference") (OtherBodyIndex :type Integer))
  (`SceneComponent.SetVisibility` (`self.Widget`) false false))

(event `self.ReceiveTick`
  (params (DeltaSeconds :type "Float (single-precision)"))
  (bind _plane (`self.Plane`))
  (bind _asbp_third_person_character (cast `/Game/ThirdPerson/Blueprints/BP_ThirdPersonCharacter` (`GameplayStatics.GetPlayerCharacter` 0)))
  (bind (_returnvalue_roll _returnvalue_pitch _returnvalue_yaw) (`KismetMathLibrary.BreakRotator` (`KismetMathLibrary.FindLookAtRotation` (`SceneComponent.K2_GetComponentLocation` _plane) (`SceneComponent.K2_GetComponentLocation` (`/Game/ThirdPerson/Blueprints/BP_ThirdPersonCharacter.FollowCamera` _asbp_third_person_character)))))
  ; Rotate 2D Plane to look at Camera
  (`SceneComponent.K2_SetWorldRotation` _plane (`KismetMathLibrary.MakeRotator` 270.0 0.0 (+ _returnvalue_yaw 90.0)) false false))

(event `self.ReceiveActorBeginOverlap`
  (params (OtherActor :type "Actor Object Reference")))

(fn `NewFunction`)

(fn `Pick Up Item`
  (returns (item :type String))
  (if true
    (`KismetSystemLibrary.PrintString` "item picked")
    (`self.Destroy Item`)
    (return (`self.item`))))

(fn `UserConstructionScript`)